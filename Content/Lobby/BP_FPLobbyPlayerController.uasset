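; Lobby player controller that shows a debug lobby screen to the local player.
; On BeginPlay it switches input to game-and-UI mode, then creates the WBP_Screen_DEBUG_Lobby widget for local controllers only and adds it to the viewport.
; The stored widget is removed from its parent when the controller is destroyed.
; Tick prints a debug label on screen every frame.
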(event `self.ReceiveTick`
  (params (DeltaSeconds :type "Float (single-precision)"))
  (`KismetSystemLibrary.PrintString` "PC_Lobby" true false (struct :`G` 0.66 :`B` 1.0 :`A` 1.0) 0.0))

(event `self.ReceiveBeginPlay`
  ;[0 0.1932 0.6281] Begin Play
  (`WidgetBlueprintLibrary.SetInputMode_GameAndUIEx` self null "DoNotLock" false)
  (`self.CreateLobbyWidget`))

(event `CreateLobbyWidget`
  ;[0 0.7537 0.06764] Create Lobby widget
  (if (`self.IsLocalPlayerController`)
    (bind _returnvalue (`|CreateWidget` "/FPLobby/Lobby/WBP_Screen_DEBUG_Lobby.WBP_Screen_DEBUG_Lobby_C" self))
    (`UserWidget.AddToViewport` _returnvalue 0)
    (set `self.LobbyWidget` _returnvalue)))

(event `self.ReceiveDestroyed`
  (`Widget.RemoveFromParent` (`self.LobbyWidget`)))

(fn `UserConstructionScript`)