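; Lobby game mode that tracks players joining and leaving a multiplayer lobby.
; After a one-second delay, login and logout fire player event dispatchers and tell BP_FPLobbyGameState to update its lobby players.
; Login also calls AddPlayer, which writes PlayerIndex on the lobby player controller from a local index that nothing here assigns.
; Helper functions gather connected players' controllers, names and unique net IDs by index.
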(event `self.K2_PostLogin`
  (params (NewPlayer :type "PlayerController Object Reference"))
  ;[0 0.03865 0.7827] Login
  (`KismetSystemLibrary.Delay` 1.0)
  (`self.AddPlayer` NewPlayer)
  (`KismetSystemLibrary.PrintString` (`KismetStringLibrary.Concat_StrStr` "OnPostLogin: " (`AdvancedSessionsLibrary.GetPlayerName` NewPlayer)))
  (`self.OnPlayerLogin` NewPlayer)
  (bind _asbp_fplobby_game_state (cast `/FPLobby/Lobby/BP_FPLobbyGameState` (`GameplayStatics.GetGameState`)))
  (`/FPLobby/Lobby/BP_FPLobbyGameState.UpdatePlayersInLobby` _asbp_fplobby_game_state))

(event `self.K2_OnLogout`
  (params (ExitingController :type "Controller Object Reference"))
  ;[0 0.7827 0.03865] Log out
  (bind _asplayer_controller (cast `PlayerController` ExitingController))
  (`KismetSystemLibrary.Delay` 1.0)
  (`KismetSystemLibrary.PrintString` (`KismetStringLibrary.Concat_StrStr` "OnLogout: " (`AdvancedSessionsLibrary.GetPlayerName` _asplayer_controller)))
  (`self.OnPlayerLogout` _asplayer_controller)
  (bind _asbp_fplobby_game_state (cast `/FPLobby/Lobby/BP_FPLobbyGameState` (`GameplayStatics.GetGameState`)))
  (`/FPLobby/Lobby/BP_FPLobbyGameState.UpdatePlayersInLobby` _asbp_fplobby_game_state))

(event `self.HandleStartingNewPlayer`
  (params (NewPlayer :type "PlayerController Object Reference"))
  ;[0 0.3092 0.5121] Start new player
  (`parent.HandleStartingNewPlayer` NewPlayer)
  (`KismetSystemLibrary.PrintString` (`KismetStringLibrary.Concat_StrStr` "Startup New Player: " (`KismetSystemLibrary.GetDisplayName` NewPlayer))))

(event `self.ReceiveBeginPlay`)

(fn `AddPlayer`
  (params (Player :type "PlayerController Object Reference"))
  (locals (LocalPlayerIndex :type Integer :default 0))
  (`|ExecutionSequence`
    (:`then_1`
      ;[0.4155 0 0.4107] Update index on player controller
      (bind _asbp_fplobby_player_controller (cast `/FPLobby/Lobby/BP_FPLobbyPlayerController` (`local.Player`)))
      (set `/FPLobby/Lobby/BP_FPLobbyPlayerController.PlayerIndex` (`local.LocalPlayerIndex`) _asbp_fplobby_player_controller))))

(fn `GetPlayerNames`
  (returns (PlayerNames :type "Array of String"))
  (locals (Names :type "Array of String"))
  (`|ExecutionSequence`
    (:`then_0`
      (for _index (range (`AdvancedSessionsLibrary.GetNumberOfNetworkPlayers`))
        (`KismetArrayLibrary.Array_Add` (`local.Names`) (`AdvancedSessionsLibrary.GetPlayerName` (`GameplayStatics.GetPlayerController` _index)))))
    (:`then_1`
      (return (`local.Names`)))))

(fn `GetPlayerNetIds`
  (returns (ReturnValue :type "Array of BPUniqueNetId Structure"))
  (locals (NetIds :type "Array of BPUniqueNetId Structure"))
  (`|ExecutionSequence`
    (:`then_0`
      (for _index (range (`AdvancedSessionsLibrary.GetNumberOfNetworkPlayers`))
        (`KismetArrayLibrary.Array_Add` (`local.NetIds`) (`AdvancedSessionsLibrary.GetUniqueNetID` (`GameplayStatics.GetPlayerController` _index)))))
    (:`then_1`
      (return (`local.NetIds`)))))

(fn `GetPlayers`
  (returns (ReturnValue :type "Array of PlayerController Object Reference"))
  (locals (Players :type "Array of PlayerController Object Reference"))
  (`|ExecutionSequence`
    (:`then_0`
      (for _index (range (`AdvancedSessionsLibrary.GetNumberOfNetworkPlayers`))
        (`KismetArrayLibrary.Array_Add` (`local.Players`) (`GameplayStatics.GetPlayerController` _index))))
    (:`then_1`
      (return (`local.Players`)))))

(fn `UserConstructionScript`)